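; Player controller for the multiplayer lobby, managing the lobby UI, chat, loading screen and leaving the session.
; On start it registers GameIN_Main's player info with GM_Lobby, creates the widgets and announces the join in chat.
; Player updates route through GM_Lobby, and chat fans out to every controller in its PlayerList.
; Leaving destroys the session and opens MAP_Start on success.
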(event `self.ReceiveBeginPlay`
  ;[1 1 1] 开始
  (`self.EVE_Init`))

(event `EVE_Init`
  ;[1 1 1] 初始化
  (bind _asgame_in_main (cast `/Game/Maple/Game/GameIN_Main` (`GameplayStatics.GetGameInstance`)))
  (bind _output_get (set `self.PlayerInfo` (`/Game/Maple/Game/GameIN_Main.PlayerInfo` _asgame_in_main)))
  (`self.EVE_AddplayerInfo` _output_get)
  (`self.EVE_ShowLobbyUI`)
  (`self.EVE_ShowChatFrame`)
  (`self.EVE_AddChatInfo` "【系统】" (`|FormatText` "玩家 {name} 进入了房间" (`.Name_5_7ADD5BB8437016A013D267ADFEE4B30D` (break `/Game/Maple/Game/Variable/Str_PlayerInfo` (`self.PlayerInfo`))))))

(event `EVE_ShowLobbyUI`
  ;[1 1 1] 创建显示大厅控件
  (set `self.bShowMouseCursor` true)
  (bind _returnvalue (`|CreateWidget` "/Game/Maple/UI/UI_Lobby.UI_Lobby_C" self))
  (bind _output_get (set `self.UI_Lobby` _returnvalue))
  (`UserWidget.AddToViewport` _output_get 0)
  (`WidgetBlueprintLibrary.SetInputMode_GameAndUIEx` self (`self.UI_Lobby`))
  (`self.EVE_UpdateAllPlayer`))

(event `EVE_UpdateAllPlayer`
  ;[1 1 1] 更新所有玩家
  (bind _asgm_lobby (cast `/Game/Maple/Game/Lobby/GM_Lobby` (`GameplayStatics.GetGameMode`)))
  (`/Game/Maple/Game/Lobby/GM_Lobby.EVE_UpdateAllPlayer` _asgm_lobby))

(event `EVE_AddplayerInfo`
  (params (PlayerInfo :type "/Game/Maple/Game/Variable/Str_PlayerInfo Structure"))
  ;[1 1 1] 添加人物信息
  (bind _asgm_lobby (cast `/Game/Maple/Game/Lobby/GM_Lobby` (`GameplayStatics.GetGameMode`)))
  (`/Game/Maple/Game/Lobby/GM_Lobby.EVE_AddPlayerInfo` _asgm_lobby PlayerInfo))

(event `EVE_UpdateSelf`
  (params (PlayerInfo :type "Array of /Game/Maple/Game/Variable/Str_PlayerInfo Structure") (CpName :type Text) (MaxPlayerQuantity :type Integer))
  (bind _ui_lobby (`self.UI_Lobby`))
  ;[1 1 1] 更新自身大厅控件信息
  (`/Game/Maple/UI/UI_Lobby.EVE_UpdateInfo` _ui_lobby PlayerInfo MaxPlayerQuantity)
  (`/Game/Maple/UI/UI_Lobby.EVE_UpdateCpName` _ui_lobby CpName))

(event `EVE_ShowLoading`
  ;[1 1 1] 创建加载
  (bind _returnvalue (`|CreateWidget` "/Game/Maple/UI/UI_Loading.UI_Loading_C" self))
  (`UserWidget.AddToViewport` _returnvalue 0))

(event `EVE_UpdatePlayerInfo`
  (params (info :type "/Game/Maple/Game/Variable/Str_PlayerInfo Structure"))
  ;[1 1 1] 更新玩家信息
  (bind _asgm_lobby (cast `/Game/Maple/Game/Lobby/GM_Lobby` (`GameplayStatics.GetGameMode`)))
  (`/Game/Maple/Game/Lobby/GM_Lobby.EVE_UpdatePlayerInfo` _asgm_lobby info))

(event `EVE_LeaveRomm`
  ;[1 1 1] 离开房间
  (`DestroySessionCallbackProxy.DestroySession` self
    (:`OnSuccess`
      (`KismetSystemLibrary.PrintString` "离开成功")
      (`GameplayStatics.OpenLevel` "MAP_Start"))
    (:`OnFailure`
      (`KismetSystemLibrary.PrintString` "离开失败"))))

(event `EVE_ShowChatFrame`
  ;[1 1 1] 聊天框
  ;;[1 1 1] 创建大厅聊天框
  (bind _returnvalue (`|CreateWidget` "/Game/Maple/UI/ChatFrame/UI_LobbyChatFrame.UI_LobbyChatFrame_C" self))
  (bind _output_get (set `self.UI_ChatFrame` _returnvalue))
  (`UserWidget.AddToViewport` _output_get 0))

(event `EVE_NewMessage`
  (params (Text :type Text))
  ;[1 1 1] 聊天框
  ;;[1 1 1] 更新新的消息
  (`/Game/Maple/UI/ChatFrame/UI_Com_ChatFrame.EVE_UpdateNewMessage` (`/Game/Maple/UI/ChatFrame/UI_LobbyChatFrame.UI_Com_ChatFrame` (`self.UI_ChatFrame`)) Text))

(event `EVE_AddChatInfo`
  (params (Before :type Text) (Text :type Text))
  ;[1 1 1] 聊天框
  ;;[1 1 1] 增加新的信息
  (bind _asgm_lobby (cast `/Game/Maple/Game/Lobby/GM_Lobby` (`GameplayStatics.GetGameMode`)))
  (for _array_element (`/Game/Maple/Game/Lobby/GM_Lobby.PlayerList` _asgm_lobby)
    (bind _aspc_lobby (cast `/Game/Maple/Game/Lobby/PC_Lobby` _array_element))
    (`self.EVE_NewMessage` _aspc_lobby (`|FormatText` "{before}：{Text}" Before Text))))

(fn `UserConstructionScript`)