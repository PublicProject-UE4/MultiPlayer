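; Lobby game mode that manages a multiplayer room's players, map info and travel to MAP_Game.
; On the server, it reads checkpoint name and room capacity from GameIN_Main, and spawns joiners as PCH_Lobby at the first PlayerStart found.
; Parallel controller and info arrays track players; logouts and info edits push the list and room settings to every PC_Lobby.
; Events also handle kicking by index and starting the game via ServerTravel.
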(event `self.K2_OnLogout`
  (params (ExitingController :type "Controller Object Reference"))
  ;[1 1 1] 玩家退出
  (`/Engine/EditorBlueprintResources/ActorMacros.Switch Has Authority`
    (:`Authority`
      (for (_array_element _array_index) (`self.PlayerList`)
        (if (== _array_element ExitingController)
          (`KismetArrayLibrary.Array_RemoveItem` (`self.PlayerList`) _array_element)
          (`KismetArrayLibrary.Array_Remove` (`self.PlayerInfoList`) _array_index)))
      (`self.EVE_UpdateAllPlayer`))))

(event `self.K2_PostLogin`
  (params (NewPlayer :type "PlayerController Object Reference"))
  ;[1 1 1] 玩家登陆
  (`/Engine/EditorBlueprintResources/ActorMacros.Switch Has Authority`
    (:`Authority`
      (`KismetArrayLibrary.Array_AddUnique` (`self.PlayerList`) NewPlayer)
      (`self.EVE_SpawnPlayer` NewPlayer))))

(event `self.ReceiveBeginPlay`
  ;[1 1 1] 获取地图信息保存到gamemode
  (`/Engine/EditorBlueprintResources/ActorMacros.Switch Has Authority`
    (:`Authority`
      (bind _asgame_in_main (cast `/Game/Maple/Game/GameIN_Main` (`GameplayStatics.GetGameInstance`)))
      (set `self.Cp_Name` (`/Game/Maple/Game/GameIN_Main.CheckpointName` _asgame_in_main))
      (set `self.MaxQuantity` (`/Game/Maple/Game/GameIN_Main.RoomMaxPlayerQuantity` _asgame_in_main)))))

(event `EVE_SpawnPlayer`
  (params (PC :type "PlayerController Object Reference"))
  (bind _returnvalue (`Controller.K2_GetPawn` PC))
  ;[1 1 1] 生成玩家
  (`/Engine/EditorBlueprintResources/StandardMacros.IsValid` _returnvalue
    (:`Is Valid`
      (`self.K2_DestroyActor` _returnvalue))
    (:`Is Not Valid`
      _))
  (bind _outactors (`GameplayStatics.GetAllActorsOfClass` "/Script/Engine.PlayerStart"))
  (bind _returnvalue_2 (`|SpawnActorFromClass` "/Game/Maple/Game/Lobby/PCH_Lobby.PCH_Lobby_C" (`KismetMathLibrary.MakeTransform` (`self.K2_GetActorLocation` (`|GetArrayItem` _outactors))) "AdjustIfPossibleButAlwaysSpawn" "OverrideRootScale" null null))
  (`Controller.Possess` PC _returnvalue_2))

(event `EVE_AddPlayerInfo`
  (params (playerinfo :type "/Game/Maple/Game/Variable/Str_PlayerInfo Structure (by ref)"))
  ;[1 1 1] 添加玩家信息
  (`KismetArrayLibrary.Array_Add` (`self.PlayerInfoList`) playerinfo))

(event `EVE_StartCp`
  ;[1 1 1] 场景漫游
  (`KismetSystemLibrary.ExecuteConsoleCommand` "ServerTravel MAP_Game" (`GameplayStatics.GetPlayerController` 0)))

(event `EVE_UpdateAllPlayer`
  ;[1 1 1] 更新所有玩家
  (for _array_element (`self.PlayerList`)
    (bind _aspc_lobby (cast `/Game/Maple/Game/Lobby/PC_Lobby` _array_element))
    (`/Game/Maple/Game/Lobby/PC_Lobby.EVE_UpdateSelf` _aspc_lobby (`self.PlayerInfoList`) (`self.Cp_Name`) (`self.MaxQuantity`))))

(event `EVE_UpdatePlayerInfo`
  (params (info :type "/Game/Maple/Game/Variable/Str_PlayerInfo Structure"))
  ;[1 1 1] 更新玩家属性
  (`KismetArrayLibrary.Array_Clear` (`self.NewPlayerInfoList`))
  (for _array_element (`self.PlayerInfoList`)
    (if (`KismetTextLibrary.EqualEqual_TextText` (`.Name_5_7ADD5BB8437016A013D267ADFEE4B30D` (break `/Game/Maple/Game/Variable/Str_PlayerInfo` _array_element)) (`.Name_5_7ADD5BB8437016A013D267ADFEE4B30D` (break `/Game/Maple/Game/Variable/Str_PlayerInfo` info)))
      (`KismetArrayLibrary.Array_Add` (`self.NewPlayerInfoList`) info)
      (else
        (`KismetArrayLibrary.Array_Add` (`self.NewPlayerInfoList`) _array_element))))
  (set `self.PlayerInfoList` (`self.NewPlayerInfoList`))
  (`self.EVE_UpdateAllPlayer`))

(event `EVE_KickPlayer`
  (params (Index :type Integer))
  ;[1 1 1] 踢出房间
  (bind _aspc_lobby (cast `/Game/Maple/Game/Lobby/PC_Lobby` (`|GetArrayItem` (`self.PlayerList`) Index)))
  (`/Game/Maple/Game/Lobby/PC_Lobby.EVE_LeaveRomm` _aspc_lobby))

(fn `UserConstructionScript`)